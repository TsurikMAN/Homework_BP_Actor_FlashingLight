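; BP_Flashing_light is a Blueprint that blinks its FLash component a set number of times when play begins.
; BeginPlay runs a Loop with Delay macro using blink interval and count variables, toggling visibility twice per blink so it ends in its initial state.
; The macro builds a delayed for-loop, waiting before each Exit pulse and firing Complited at the end, which is left unused here.
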(event EventBeginPlay
  (Utilities|LoopwithDelay 1 (Variables|Default|GetИнтервал%20Мерцаний%20%28сек%29) (* (Variables|Default|GetКоличество%20Мерцаний) 2)
    (:Exit
      (Rendering|ToggleVisibility (Variables|Default|GetFLash) false))))

(fn ConstructionScript)